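; Base power-up Blueprint: an animated pickup that a VRCharacter collects by overlapping it.
; The construction script caches the mesh's relative Z, and BeginPlay starts a timeline from a random time that bobs SceneAnimation on a sine track and spins its yaw, desyncing instances.
; Overlap is handled only with authority, where PickupEffects plays a 2D sound and destroys the actor, with no power-up effect applied here.
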(event Custom|StartAnimation
  (bind _sceneanimation (Variables|Default|GetSceneAnimation))
  ;[1 1 1] Animation
  (switch int (Variables|Default|GetAnimationType)
    (:Default
      _)
    (:0
      _))
  (Utilities|FlowControl|Sequence
    (:then_0
      (bind (_direction _sine _rotation) (Timeline|Animation SetNewTime)
        (:Update
          (Transformation|SetRelativeLocation _sceneanimation (Math|Vector|MakeVector 0.0 0.0 (+ (Variables|Default|GetInitialZLocation) (* _sine (Variables|Default|GetAnimationStrength)))) false false)
          (Transformation|SetRelativeRotation _sceneanimation (Math|Rotator|MakeRotator 0.0 0.0 _rotation) false false))))
    (:then_1
      (Timeline|Animation Play))))

(event Custom|PickupEffects
  (Audio|PlaySound2D (Variables|Default|GetPickupSound) 1.0 1.0 0.0 0 0)
  (Actor|DestroyActor))

(event EventBeginPlay
  (CallFunction|StartAnimation))

(event Collision|EventActorBeginOverlap
  (params (OtherActor :type Actor%20Object%20Reference))
  ;[1 1 1] Overlap
  (Networking|SwitchHasAuthority
    (:Authority
      (Utilities|Casting|CastToVRCharacter OtherActor)
      (CallFunction|PickupEffects))))

(fn ConstructionScript
  (Variables|Default|SetInitialZLocation (.Z (Math|Vector|BreakVector (Variables|/Script/Engine.SceneComponent|GetRelativeLocation (Variables|Default|GetStaticMesh))))))