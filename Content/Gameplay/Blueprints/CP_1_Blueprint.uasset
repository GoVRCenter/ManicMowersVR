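; Race checkpoint Blueprint that tracks checkpoint progress, lap count and elapsed time.
; A single collision component hops through an array of nine marker meshes each time an overlap ends, with a delayed DoOnce reset debouncing hits.
; After the last checkpoint it increments the lap and returns to the start while laps remain.
; Once RaceStart is set, Tick plays two looping Timelines as race and lap minute/second clocks.
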(event OnComponentEndOverlap(CollisionComp)
  (params (OverlappedComponent :type Primitive%20Component%20Object%20Reference) (OtherActor :type Actor%20Object%20Reference) (OtherComp :type Primitive%20Component%20Object%20Reference) (OtherBodyIndex :type Integer))
  (if (== (Variables|Default|GetCP_Count) 9)
    (Utilities|FlowControl|Delay 0.2)
    (Variables|Default|SetCP_Count 1)
    (bind _result (Math|Integer|IncrementInt (Variables|Default|GetLap_Count))
      (:%20%20
        (Variables|Default|SetLap_Count _result)
        (if (<= (Variables|Default|GetLap_Count) (Variables|Default|GetMax_Laps))
          ;[1 1 1] Moves collision CP to Start
          (Transformation|SetWorldTransform (Variables|Default|GetCollisionComp) (Transformation|GetWorldTransform (Variables|Default|GetStaticMeshComponent0)) false false))))
    (else
      (Utilities|FlowControl|DoOnce false :!label _label
        (:Completed
          (Transformation|SetWorldTransform (Variables|Default|GetCollisionComp) (Transformation|GetWorldTransform (Utilities|Array|Get(acopy) (Utilities|Array|MakeArray (Variables|Default|GetStaticMeshComponent0) (Variables|Default|GetStaticMeshComponent01) (Variables|Default|GetStaticMeshComponent02) (Variables|Default|GetStaticMeshComponent04) (Variables|Default|GetStaticMeshComponent05) (Variables|Default|GetStaticMeshComponent06) (Variables|Default|GetStaticMeshComponent07) (Variables|Default|GetStaticMeshComponent08) (Variables|Default|GetStaticMeshComponent09)) (Variables|Default|GetCP_Count))) false false)
          (bind _result_2 (Math|Integer|IncrementInt (Variables|Default|GetCP_Count))
            (:%20%20
              (Variables|Default|SetCP_Count _result_2)
              (Utilities|FlowControl|Delay 0.2)
              (goto _label Reset))))))))

(event EventBeginPlay)

(event Collision|EventActorBeginOverlap
  (params (OtherActor :type Actor%20Object%20Reference)))

(event EventTick
  (params (DeltaSeconds :type Float%20%28single-precision%29))
  (if (Variables|Default|GetRaceStart)
    (Utilities|FlowControl|Sequence
      (:then_0
        (bind _time_seconds (Timeline|RaceTime Play)
          (:Update
            (Variables|Default|SetSeconds _time_seconds))
          (:Finished
            (Variables|Default|SetMins (+ (Variables|Default|GetMins) 1))
            (Timeline|RaceTime PlayFromStart))))
      (:then_1
        (bind _time_seconds_2 (Timeline|LapTime Play)
          (:Update
            (Variables|Default|SetLapSeconds _time_seconds_2))
          (:Finished
            (Variables|Default|SetLapMins (+ (Variables|Default|GetLapMins) 1))
            (Timeline|LapTime PlayFromStart)))))))

(fn ConstructionScript)