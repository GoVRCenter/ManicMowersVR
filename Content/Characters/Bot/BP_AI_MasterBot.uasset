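; AI bot driver that spawns a MowerV2 at its capsule, takes the driver's seat and follows a randomly chosen BP_AI_Master_Path spline.
; A delayed Tick turns the Head toward the spline point nearest LookAhead and converts its relative yaw into steering.
; Throttle comes from clamped spline tangent length, reduced when the Box overlaps more than one mower.
; Brake calls are unconnected.
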(event EventBeginPlay
  (bind _self self)
  (bind _capsulecomponent (Variables|Default|GetCapsuleComponent))
  (bind _returnvalue (Transformation|GetWorldLocation _capsulecomponent))
  (Utilities|FlowControl|Sequence
    (:then_0
      ;[1 1 1] Place Bot into vehicle
      (bind _returnvalue_2 (Game|SpawnActorfromClass "/Game/VRExpansion/Vive/Testing/Car/VehicleBP/Sedan/MowerV2.MowerV2_C" (Math|Transform|MakeTransform (Math|Vector|MakeVector (.x _returnvalue) (.y _returnvalue) (- (.z _returnvalue) (Variables|/Script/Engine.CapsuleComponent|GetCapsuleHalfHeight _capsulecomponent))) (Transformation|GetWorldRotation _capsulecomponent)) "AlwaysSpawn" _self _self))
      (bind _output_get (Variables|Default|SetVehicle _returnvalue_2))
      (Default|ForcePlayerIntoDriversSeat _output_get _self))
    (:then_1
      ;[1 1 1] Find all possible routes through the track
      (bind _outactors (Actor|GetAllActorsOfClass "/Game/Gameplay/Blueprints/BP_AI_Master_Path.BP_AI_Master_Path_C"))
      (for _array_element _outactors
        (bind _returnvalue_3 (Utilities|Array|Add (Variables|Default|GetSplinePaths) _array_element))
        (Variables|Default|SetCurrentPath _returnvalue_3))
      (Variables|Default|SetCurrentPath (Math|Random|RandomIntegerinRange 0 (Variables|Default|GetCurrentPath))))))

(event EventTick
  (params (DeltaSeconds :type Float%20%28single-precision%29))
  (bind _vehicle (Variables|Default|GetVehicle))
  (bind _currentpath (Variables|Default|GetCurrentPath))
  (bind _lookahead (Variables|Default|GetLookAhead))
  (bind _splinepaths (Variables|Default|GetSplinePaths))
  (bind _head (Variables|Default|GetHead))
  (bind _returnvalue (Transformation|GetWorldLocation _lookahead))
  (bind _output (Utilities|Array|Get(acopy) _splinepaths _currentpath))
  (bind _vehiclemovement (Variables|/Script/PhysXVehicles.WheeledVehicle|GetVehicleMovement _vehicle))
  (bind _splinepath (Variables|/Game/Gameplay/Blueprints/BP_AI_Master_Path.BP_AI_Master_Path_C|GetSplinePath _output))
  (bind _returnvalue_2 (Class|SplineComponent|FindTangentClosesttoWorldLocation _splinepath _returnvalue "World"))
  (bind _returnvalue_3 (Math|Vector|VectorLength _returnvalue_2))
  (bind _returnvalue_4 (Math|Float|Clamp(Float) _returnvalue_3 0.0 0.96))
  ;[1 0.291 0.3208] Sloppy Control updating...
  (Utilities|FlowControl|Delay 0.04)
  (Transformation|SetWorldRotation _head (Math|Rotator|FindLookatRotation (Transformation|GetWorldLocation (Variables|Default|GetCapsuleComponent)) (Spline|FindLocationClosesttoWorldLocation _splinepath _returnvalue "World")) false false)
  (Class|WheeledVehicleMovementComponent|SetSteeringInput (Variables|/Script/PhysXVehicles.WheeledVehicle|GetVehicleMovement (Variables|Default|GetVehicle)) (Math|Float|Clamp(Float) (* (.yaw (Variables|/Script/Engine.SceneComponent|GetRelativeRotation _head)) 0.01) -1.0))
  (if (> (Utilities|Array|Length (Collision|GetOverlappingActors (Variables|Default|GetBox) "/Game/VRExpansion/Vive/Testing/Car/VehicleBP/Sedan/MowerV2.MowerV2_C" :!class /Script/Engine.PrimitiveComponent)) 1)
    (Class|WheeledVehicleMovementComponent|SetThrottleInput _vehiclemovement (* _returnvalue_4 0.65))
    (else
      (Class|WheeledVehicleMovementComponent|SetThrottleInput _vehiclemovement _returnvalue_4))))

(fn ConstructionScript)